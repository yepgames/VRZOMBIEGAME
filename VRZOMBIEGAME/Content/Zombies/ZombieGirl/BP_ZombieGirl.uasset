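; BP_ZombieGirl is a zombie enemy that chases the player and plays an attack montage on reaching them.
; From BeginPlay it runs AI MoveTo toward the player controller (not the pawn), retrying on failure.
; A successful move triggers the attack montage, whose completion restarts the chase; no damage is applied here.
; PawnSensing sight only raises walk speed, which is never lowered again.
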(event `self.PawnSensing.OnSeePawn`
  (params (Pawn :type "Pawn Object Reference"))
  (set `CharacterMovementComponent.MaxWalkSpeed` 360.0 (`self.CharacterMovement`)))

(event `self.ReceiveBeginPlay`
  (`self.runtoplayer`))

(event `runtoplayer`
  (`|AIMoveTo` self (0.0 0.0 0.0) (`GameplayStatics.GetPlayerController` 0) 40.0
    (:`OnSuccess`
      (`self.attackplayer`))
    (:`OnFail`
      (`self.runtoplayer`))))

(event `attackplayer`
  (`|PlayMontage` (`self.Mesh`) "/Game/Zombies/ZombieGirl/Animations/zombie_attack_Montage.zombie_attack_Montage"
    (:`OnCompleted`
      (`self.runtoplayer`))))

(fn `UserConstructionScript`)