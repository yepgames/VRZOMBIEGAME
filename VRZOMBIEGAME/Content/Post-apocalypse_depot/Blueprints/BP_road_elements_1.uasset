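; BP_road_elements_1 is a construction-script Blueprint that lays road element meshes along an editable spline in the depot environment.
; It scales SectionLength by the actor's X scale, then adds one X-forward spline mesh component per whole section that fits the spline.
; Each segment takes its endpoints and tangents from the spline, with tangents clamped to section length and query-and-physics collision enabled.
; Any leftover length shorter than a section stays uncovered.
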(fn `UserConstructionScript`
  (bind _returnvalue_x (`KismetMathLibrary.BreakVector` (`self.GetActorScale3D`)))
  (bind _spline (`self.Spline`))
  (`|ExecutionSequence`
    (:`then_0`
      (set `self.SectionLength` (* _returnvalue_x (`self.SectionLength`)))
      (for _index (range (`KismetMathLibrary.FTrunc` (/ (`SplineComponent.GetSplineLength` (`self.Spline`)) (`self.SectionLength`))))
        (bind _returnvalue (`AddComponent|NODE_AddSplineMeshComponent-2`))
        (`SplineMeshComponent.SetForwardAxis` _returnvalue "X" true)
        (bind _returnvalue_2 (* _index (`self.SectionLength`)))
        (bind _returnvalue_3 (* (+ _index 1) (`self.SectionLength`)))
        (`SplineMeshComponent.SetStartAndEnd` _returnvalue (`SplineComponent.GetLocationAtDistanceAlongSpline` _spline _returnvalue_2 "Local") (`KismetMathLibrary.ClampVectorSize` (`SplineComponent.GetTangentAtDistanceAlongSpline` _spline _returnvalue_2 "Local") 0.0 (`self.SectionLength`)) (`SplineComponent.GetLocationAtDistanceAlongSpline` _spline _returnvalue_3 "Local") (`KismetMathLibrary.ClampVectorSize` (`SplineComponent.GetTangentAtDistanceAlongSpline` _spline _returnvalue_3 "Local") 0.0 (`self.SectionLength`)) true)
        (`PrimitiveComponent.SetCollisionEnabled` _returnvalue "QueryAndPhysics")))))