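; Construction-script Blueprint that bends a static mesh along a spline, apparently for ivy on railway poles in the depot environment, judging by its name.
; It adds one spline mesh component per segment, matching local point positions and tangents, with a variable forward axis and query-and-physics collision.
; An unconnected branch that would place road element meshes at fixed spacing along the spline never runs.
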(fn `UserConstructionScript`
  (bind _spline (`self.Spline`))
  (bind _spline_2 (`self.Spline`))
  (`|ExecutionSequence`
    (:`then_0`
      (for _index (range (+ (- (`SplineComponent.GetNumberOfSplinePoints` _spline_2) 2) 1))
        (bind _returnvalue (`AddComponent|NODE_AddSplineMeshComponent-2`))
        (`StaticMeshComponent.SetStaticMesh` _returnvalue (`self.static mesh`))
        (`PrimitiveComponent.SetMaterial` _spline_2 0 null)
        (`SplineMeshComponent.SetForwardAxis` _returnvalue (`self.axis`) true)
        (`SceneComponent.K2_AttachToComponent` _returnvalue _spline_2 "None" "KeepRelative" "KeepRelative" "KeepRelative" true)
        (bind _returnvalue_2 (+ _index 1 0))
        (`SplineMeshComponent.SetStartAndEnd` _returnvalue (`SplineComponent.GetLocationAtSplinePoint` _spline _index "Local") (`SplineComponent.GetTangentAtSplinePoint` _spline _index "Local") (`SplineComponent.GetLocationAtSplinePoint` _spline _returnvalue_2 "Local") (`SplineComponent.GetTangentAtSplinePoint` _spline _returnvalue_2 "Local") true)
        (`PrimitiveComponent.SetCollisionEnabled` _returnvalue "QueryAndPhysics")))))