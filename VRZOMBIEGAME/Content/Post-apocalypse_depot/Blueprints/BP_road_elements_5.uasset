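; BP_road_elements_5 is a spline-driven construction-script Blueprint that builds a run of road elements for the post-apocalyptic depot environment.
; It lays deforming spline meshes in sections whose length scales with actor X scale, clamping tangents to the section length.
; A second pass places SM_road_elements_11 connector meshes at fixed spacing, rotated to follow the spline.
; Both sets of generated components get query and physics collision.
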(fn `UserConstructionScript`
  (bind _returnvalue_x (`KismetMathLibrary.BreakVector` (`self.GetActorScale3D`)))
  (bind _spline (`self.Spline`))
  (bind _spline_2 (`self.Spline`))
  (bind _spacing (`self.Spacing`))
  (`|ExecutionSequence`
    (:`then_0`
      (set `self.SectionLength` (* _returnvalue_x (`self.SectionLength`)))
      (for _index (range (`KismetMathLibrary.FTrunc` (/ (`SplineComponent.GetSplineLength` _spline) (`self.SectionLength`))))
        (bind _returnvalue (`AddComponent|NODE_AddSplineMeshComponent-2`))
        (`SplineMeshComponent.SetForwardAxis` _returnvalue "X" true)
        (bind _returnvalue_2 (* _index (`self.SectionLength`)))
        (bind _returnvalue_3 (* (+ _index 1) (`self.SectionLength`)))
        (`SplineMeshComponent.SetStartAndEnd` _returnvalue (`SplineComponent.GetLocationAtDistanceAlongSpline` _spline_2 _returnvalue_2 "Local") (`KismetMathLibrary.ClampVectorSize` (`SplineComponent.GetTangentAtDistanceAlongSpline` _spline_2 _returnvalue_2 "Local") 0.0 (`self.SectionLength`)) (`SplineComponent.GetLocationAtDistanceAlongSpline` _spline_2 _returnvalue_3 "Local") (`KismetMathLibrary.ClampVectorSize` (`SplineComponent.GetTangentAtDistanceAlongSpline` _spline_2 _returnvalue_3 "Local") 0.0 (`self.SectionLength`)) true)
        (`PrimitiveComponent.SetCollisionEnabled` _returnvalue "QueryAndPhysics")))
    (:`then_1`
      ;[1 1 1] Sigment of connect
      (for _index_2 (range (+ (`.ReturnValue` (`KismetMathLibrary.FMod` (`SplineComponent.GetSplineLength` _spline) _spacing)) 1))
        (bind _returnvalue_4 (* _index_2 _spacing))
        (bind _returnvalue_5 (`AddComponent|NODE_AddStaticMeshComponent-4` :`RelativeTransform` (`KismetMathLibrary.MakeTransform` (`SplineComponent.GetLocationAtDistanceAlongSpline` _spline _returnvalue_4 "Local") (`SplineComponent.GetRotationAtDistanceAlongSpline` _spline _returnvalue_4 "Local"))))
        (`StaticMeshComponent.SetStaticMesh` _returnvalue_5 "/Game/Post-apocalypse_depot/Meshes/road_elements/SM_road_elements_11.SM_road_elements_11")
        (`PrimitiveComponent.SetCollisionEnabled` _returnvalue_5 "QueryAndPhysics")))))